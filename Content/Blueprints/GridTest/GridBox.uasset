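; GridBox is a test actor that visualizes a grid of debug boxes sized by its Width and Height variables.
; Tick calls DrawGrid, whose nested inclusive loops redraw short-lived boxes every frame at fixed spacing.
; The grid starts at world origin in X and Y, taking only its height from the actor.
; The construction script holds a disconnected copy of the drawing loop that never runs.
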(event EventBeginPlay)

(event Collision|EventActorBeginOverlap
  (params (OtherActor :type Actor%20Object%20Reference)))

(event EventTick
  (params (DeltaSeconds :type Float%20%28single-precision%29))
  (CallFunction|DrawGrid DeltaSeconds))

(fn ConstructionScript)

(fn DrawGrid
  (params (delta :type Float%20%28single-precision%29))
  (for _index (range 0 (Variables|Default|GetWidth))
    (for _index_2 (range 0 (Variables|Default|GetHeight))
      (Rendering|Debug|DrawDebugBox :Center (Math|Vector|MakeVector (* _index 1e+02) (* _index_2 1e+02) (.Z (Math|Vector|BreakVector (Transformation|GetActorLocation)))) :Extent (Math|Vector|MakeVector 45.0 45.0 45.0) :Duration 0.1 :Thickness 2.0))))