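; GridController is an actor that builds a grid of GridBase actors centred on its own location when play begins.
; Nested loops over twice the Rows and Columns values use Multiplier to turn each index into a signed offset at 100-unit spacing.
; Each spawned cell shares the controller's height and is stored in GridArray.
; Spawning happens at BeginPlay, leaving the construction script empty.
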(event EventBeginPlay
  (bind _returnvalue (Transformation|GetActorLocation))
  (bind _rows (Variables|Default|GetRows))
  (bind _columns (Variables|Default|GetColumns))
  (bind (_x _y _z) (Math|Vector|BreakVector _returnvalue))
  ;[1 1 1] Should be doing it here, not in the constructio script
  (for _index (range 0 (* _rows 2))
    (for _index_2 (range 0 (* _columns 2))
      (bind _returnvalue_2 (Game|SpawnActorfromClass "/Game/Blueprints/GridTest/GridBase.GridBase_C" (Math|Conversions|ToTransform(Vector) (Math|Vector|MakeVector (+ (CallFunction|Multiplier _index _rows) _x) (+ (CallFunction|Multiplier _index_2 _columns) _y) _z)) "Undefined" 0 0))
      (Utilities|Array|Add (Variables|Default|GetGridArray) _returnvalue_2))))

(fn ConstructionScript)

(fn Multiplier
  (params (Index :type Integer) (Size :type Integer))
  (return (* (- Index Size) 1e+02)))